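; Paper2D boar enemy that patrols by flipping around when its wall detector begins an overlap or its ledge detector ends one.
; PlayerDetector overlap begin and end both call ChargeAnimation, which can switch to a non-looping run flipbook when grounded and set InSightRange.
; When a flipbook finishes, it restarts the walk animation and clears that flag.
; MoveForward supplies movement input but has no caller here, and the HitCheck damage function is never run.
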(event `MoveForward`
  (`self.AddMovementInput` (* (`self.GetActorForwardVector`) (-1.0 0.0 0.0))))

(event `self.WallDetector.OnComponentBeginOverlap`
  (params (OverlappedComponent :type "PrimitiveComponent Object Reference") (OtherActor :type "Actor Object Reference") (OtherComp :type "PrimitiveComponent Object Reference") (OtherBodyIndex :type Integer) (bFromSweep :type Boolean) (SweepResult :type "HitResult Structure (by ref)"))
  (`self.TurnChar`))

(event `self.Ledge Detector.OnComponentEndOverlap`
  (params (OverlappedComponent :type "PrimitiveComponent Object Reference") (OtherActor :type "Actor Object Reference") (OtherComp :type "PrimitiveComponent Object Reference") (OtherBodyIndex :type Integer))
  (`self.TurnChar`))

(event `self.ReceiveTick`
  (params (DeltaSeconds :type "Float (single-precision)")))

(event `self.PlayerDetector.OnComponentBeginOverlap`
  (params (OverlappedComponent :type "PrimitiveComponent Object Reference") (OtherActor :type "Actor Object Reference") (OtherComp :type "PrimitiveComponent Object Reference") (OtherBodyIndex :type Integer) (bFromSweep :type Boolean) (SweepResult :type "HitResult Structure (by ref)"))
  (`self.Charge Animation`))

(event `self.PlayerDetector.OnComponentEndOverlap`
  (params (OverlappedComponent :type "PrimitiveComponent Object Reference") (OtherActor :type "Actor Object Reference") (OtherComp :type "PrimitiveComponent Object Reference") (OtherBodyIndex :type Integer))
  (`self.Charge Animation`))

(event `self.Sprite.OnFinishedPlaying`
  (`PaperFlipbookComponent.SetFlipbook` (`self.Sprite`) "/Game/PaperAssets/Mob/Boar/Walk/Flipbooks/FB_Walk_Boar1.FB_Walk_Boar1")
  (`PaperFlipbookComponent.SetLooping` (`self.Sprite`) false)
  (`self.RestartAttackAnimation`)
  (set `self.InSightRange` false))

(fn `Charge Animation`
  (if (`NavMovementComponent.IsMovingOnGround` (`self.CharacterMovement`))
    (for _ (`PrimitiveComponent.GetOverlappingActors` (`self.PlayerDetector`) "BP_EnemyBoar_C")
      _)
    (if (!= null self)
      (`PaperFlipbookComponent.SetFlipbook` (`self.Sprite`) "/Game/PaperAssets/Mob/Boar/Run/Flipbooks/FB_Run1.FB_Run1")
      (`PaperFlipbookComponent.SetLooping` (`self.Sprite`) false)
      (set `self.InSightRange` true))))

(fn `HitCheck`
  (locals (HitSomething :type Boolean))
  (for _array_element (`PrimitiveComponent.GetOverlappingActors` (`self.Hitbox`) "/Script/Engine.Actor")
    (if (!= _array_element self)
      (`GameplayStatics.ApplyDamage` _array_element (`self.DamageAmount`)))))

(fn `RestartAttackAnimation`
  (if (not (`PaperFlipbookComponent.IsPlaying` (`self.Sprite`)))
    (`PaperFlipbookComponent.Play` (`self.Sprite`))))

(fn `TurnChar`
  (`self.K2_SetActorRotation` (`KismetMathLibrary.ComposeRotators` (`self.K2_GetActorRotation`) (struct :`Yaw` 180.0))))

(fn `UserConstructionScript`)